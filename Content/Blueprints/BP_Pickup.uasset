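; BP_Pickup is a collectible actor that the third-person character picks up by overlapping it.
; On overlap it increments the character's CollectItem counter and prints the new total to the screen.
; It then toggles the Pickup component's visibility, disables its collision, and destroys itself after a short delay.
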(event `self.ReceiveActorBeginOverlap`
  (params (OtherActor :type "Actor Object Reference"))
  (bind _pickup (`self.Pickup`))
  (bind _asbp_third_person_character (cast `/Game/ThirdPerson/Blueprints/BP_ThirdPersonCharacter` OtherActor))
  (`/Engine/EditorBlueprintResources/StandardMacros.IsValid` _asbp_third_person_character
    (:`Is Valid`
      (bind _output_get (set `/Game/ThirdPerson/Blueprints/BP_ThirdPersonCharacter.CollectItem` (+ (`/Game/ThirdPerson/Blueprints/BP_ThirdPersonCharacter.CollectItem` _asbp_third_person_character) 1.0) _asbp_third_person_character))
      (`KismetSystemLibrary.PrintString` (`KismetStringLibrary.Conv_DoubleToString` _output_get))
      ;[1 1 1] Cleanup
      (`SceneComponent.ToggleVisibility` _pickup false)
      (`PrimitiveComponent.SetCollisionEnabled` _pickup "NoCollision")
      (`KismetSystemLibrary.Delay` 0.2)
      (`self.K2_DestroyActor`))))

(fn `UserConstructionScript`)