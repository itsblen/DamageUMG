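; A temporary damageable target actor that loses health when hit, shows its damage through color, and disappears at zero health.
; BeginPlay creates a dynamic damage material on the mesh and caches its Emissive color as the healthy color.
; AnyDamage calls TakeDamage, which clamps Health, blends Emissive toward HurtColor by health ratio, and hides the mesh and disables its collision at zero.
; Each hit also prints the remaining Health.
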(event `self.ReceiveBeginPlay`
  (bind _returnvalue (`KismetMaterialLibrary.CreateDynamicMaterialInstance` "/Game/Materials/M_Damage_Base_Inst.M_Damage_Base_Inst"))
  (bind _output_get (set `self.MaterialDynamic` _returnvalue))
  (`PrimitiveComponent.SetMaterial` (`self.StaticMesh`) 0 _output_get)
  (bind _returnvalue_2 (`MaterialInstanceDynamic.K2_GetVectorParameterValue` _output_get "Emissive"))
  (set `self.DefaultHealthyColor` _returnvalue_2))

(event `self.ReceiveAnyDamage`
  (params (Damage :type "Float (single-precision)") (DamageType :type "DamageType Object Reference") (InstigatedBy :type "Controller Object Reference") (DamageCauser :type "Actor Object Reference"))
  (`self.TakeDamage` Damage)
  (`KismetSystemLibrary.PrintString` (`KismetStringLibrary.Conv_DoubleToString` (`self.Health`))))

(fn `TakeDamage`
  (params (Damage :type "Float (double-precision)"))
  (bind _staticmesh (`self.StaticMesh`))
  (bind _output_get (set `self.Health` (`KismetMathLibrary.FClamp` (- (`self.Health`) Damage) 0.0 (`self.MaxHealth`))))
  (`self.UpdateDamageHighlight`)
  (if (== _output_get 0.0)
    (`SceneComponent.SetVisibility` _staticmesh false false)
    (`PrimitiveComponent.SetCollisionEnabled` _staticmesh "NoCollision")))

(fn `UpdateDamageHighlight`
  (`MaterialInstanceDynamic.SetVectorParameterValue` (`self.MaterialDynamic`) "Emissive" (`KismetMathLibrary.LinearColorLerp` (`self.HurtColor`) (`self.DefaultHealthyColor`) (`KismetMathLibrary.FClamp` (/ (`self.Health`) (`self.MaxHealth`)) 0.0 100.0))))

(fn `UserConstructionScript`)